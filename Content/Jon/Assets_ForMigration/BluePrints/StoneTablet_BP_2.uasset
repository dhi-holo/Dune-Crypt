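; StoneTablet_BP_2 is a stone tablet actor that highlights itself as selected while the player character overlaps its mesh.
; Overlap begin applies the Selected overlay material and sets actor and component tags to ST; overlap end clears the overlay and sets them to UST.
; On BeginPlay it binds DOS to a CH_Actor player event dispatcher, letting the character clear the overlay without changing the tags.
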(event `self.ReceiveBeginPlay`
  (bind _asch_actor (cast `/Game/Self/Character/CH_Actor` (`GameplayStatics.GetPlayerCharacter` 0)))
  (add `/Game/Self/Character/CH_Actor.DO` _asch_actor (delegate `DOS`)))

(event `DOS`
  (`MeshComponent.SetOverlayMaterial` (`self.StaticMesh`) null))

(event `self.StaticMesh.OnComponentBeginOverlap`
  (params (OverlappedComponent :type "PrimitiveComponent Object Reference") (OtherActor :type "Actor Object Reference") (OtherComp :type "PrimitiveComponent Object Reference") (OtherBodyIndex :type Integer) (bFromSweep :type Boolean) (SweepResult :type "HitResult Structure (by ref)"))
  (bind _st (`self.ST`))
  ;[1 1 1] Resuable Select Object
  (if (== OtherActor (`GameplayStatics.GetPlayerCharacter` 0))
    (`MeshComponent.SetOverlayMaterial` (`self.StaticMesh`) "/Game/Self/Textures/Selected.Selected")
    (set `self.Tags` _st)
    (set `ActorComponent.ComponentTags` _st (`self.StaticMesh`))))

(event `self.StaticMesh.OnComponentEndOverlap`
  (params (OverlappedComponent :type "PrimitiveComponent Object Reference") (OtherActor :type "Actor Object Reference") (OtherComp :type "PrimitiveComponent Object Reference") (OtherBodyIndex :type Integer))
  (bind _ust (`self.UST`))
  ;[1 1 1] Resuable Select Object
  (if (== OtherActor (`GameplayStatics.GetPlayerCharacter` 0))
    (`MeshComponent.SetOverlayMaterial` (`self.StaticMesh`) null)
    (set `self.Tags` _ust)
    (set `ActorComponent.ComponentTags` _ust (`self.StaticMesh`))))

(fn `UserConstructionScript`)