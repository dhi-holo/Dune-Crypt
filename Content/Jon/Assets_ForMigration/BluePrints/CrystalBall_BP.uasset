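; Crystal ball puzzle actor that displays random glyphs and highlights itself with a tag while the player overlaps it.
; A gated one-second loop picks glyph materials from a map by built name until the CG event, bound through CH_Actor, closes it.
; One trigger box reveals magic circles and another relocates the player far below.
; CG destroys those circles and the relocation box, then shows a final circle.
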(event `self.StaticMesh.OnComponentBeginOverlap`
  (params (OverlappedComponent :type "PrimitiveComponent Object Reference") (OtherActor :type "Actor Object Reference") (OtherComp :type "PrimitiveComponent Object Reference") (OtherBodyIndex :type Integer) (bFromSweep :type Boolean) (SweepResult :type "HitResult Structure (by ref)"))
  ;[1 1 1] set select object when interactable so player code can find it
  (if (== OtherActor (`GameplayStatics.GetPlayerCharacter` 0))
    (`MeshComponent.SetOverlayMaterial` (`self.StaticMesh`) "/Game/Self/Textures/Selected.Selected")
    (set `self.Tags` (`self.ST`))))

(event `self.StaticMesh.OnComponentEndOverlap`
  (params (OverlappedComponent :type "PrimitiveComponent Object Reference") (OtherActor :type "Actor Object Reference") (OtherComp :type "PrimitiveComponent Object Reference") (OtherBodyIndex :type Integer))
  ;[1 1 1] set select object when interactable so player code can find it
  (if (== OtherActor (`GameplayStatics.GetPlayerCharacter` 0))
    (`MeshComponent.SetOverlayMaterial` (`self.StaticMesh`) null)
    (set `self.Tags` (`self.UST`))))

(event `NextGlyph`
  (`PrimitiveComponent.SetMaterial` (`self.Cube`) 0 (`BlueprintMapLibrary.Map_Find` (`self.MaterialMap`) (`KismetStringLibrary.Concat_StrStr` "G" (`KismetStringLibrary.Conv_IntToString` (`self.Show`)))))
  (`KismetSystemLibrary.Delay` 1.0)
  (`self.Set Glyph`))

(event `self.ReceiveBeginPlay`
  (`SceneComponent.SetVisibility` (`self.P_ky_magicCircle2`) false false)
  (`SceneComponent.SetVisibility` (`self.P_ky_magicCircle3`) false false)
  (`SceneComponent.SetVisibility` (`self.P_ky_magicCircle4`) false false)
  (`SceneComponent.SetVisibility` (`self.P_ky_magicCircle5`) false false)
  (`SceneComponent.SetVisibility` (`self.P_ky_magicCircle6`) false false)
  (bind _asch_actor (cast `/Game/Self/Character/CH_Actor` (`GameplayStatics.GetPlayerCharacter` 0)))
  (add `/Game/Self/Character/CH_Actor.CB` _asch_actor (delegate `CG`))
  (`self.Set Glyph`))

(event `CG`
  (`|ExecutionSequence`
    (:`then_0`
      (goto _label :!via `Close`))
    (:`then_1`
      (`SceneComponent.SetVisibility` (`self.P_ky_magicCircle1`) true false)
      (`ActorComponent.K2_DestroyComponent` (`self.P_ky_magicCircle2`))
      (`ActorComponent.K2_DestroyComponent` (`self.P_ky_magicCircle3`))
      (`ActorComponent.K2_DestroyComponent` (`self.P_ky_magicCircle4`))
      (`ActorComponent.K2_DestroyComponent` (`self.P_ky_magicCircle5`))
      (`ActorComponent.K2_DestroyComponent` (`self.P_ky_magicCircle6`))
      (`ActorComponent.K2_DestroyComponent` (`self.Box2`)))))

(event `Set Glyph`
  (`/Engine/EditorBlueprintResources/StandardMacros.Gate` false :!label _label
    (:`Exit`
      (set `self.Show` (`KismetMathLibrary.RandomInteger` 10))
      (`self.NextGlyph`))))

(event `self.Box2.OnComponentBeginOverlap`
  (params (OverlappedComponent :type "PrimitiveComponent Object Reference") (OtherActor :type "Actor Object Reference") (OtherComp :type "PrimitiveComponent Object Reference") (OtherBodyIndex :type Integer) (bFromSweep :type Boolean) (SweepResult :type "HitResult Structure (by ref)"))
  (bind _returnvalue (`GameplayStatics.GetPlayerCharacter` 0))
  (if (== OtherActor _returnvalue)
    (bind _asch_actor (cast `/Game/Self/Character/CH_Actor` _returnvalue))
    (`SceneComponent.K2_SetWorldLocation` (`Character.CapsuleComponent` _asch_actor) (0.0 0.0 -4950.0) false false)))

(event `self.Box.OnComponentBeginOverlap`
  (params (OverlappedComponent :type "PrimitiveComponent Object Reference") (OtherActor :type "Actor Object Reference") (OtherComp :type "PrimitiveComponent Object Reference") (OtherBodyIndex :type Integer) (bFromSweep :type Boolean) (SweepResult :type "HitResult Structure (by ref)"))
  (if (== OtherActor (`GameplayStatics.GetPlayerCharacter` 0))
    (`SceneComponent.SetVisibility` (`self.P_ky_magicCircle2`) true false)
    (`SceneComponent.SetVisibility` (`self.P_ky_magicCircle3`) true false)
    (`SceneComponent.SetVisibility` (`self.P_ky_magicCircle4`) true false)
    (`SceneComponent.SetVisibility` (`self.P_ky_magicCircle5`) true false)
    (`SceneComponent.SetVisibility` (`self.P_ky_magicCircle6`) true false)))

(fn `UserConstructionScript`)