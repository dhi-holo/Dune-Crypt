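; Selectable knife actor that highlights itself while the player character overlaps it.
; Overlap begin applies the Selected overlay material, sets actor and component tags to ST and shows the player's KCT component on CH_Actor.
; Overlap end clears the overlay, switches the tags to UST and hides KCT.
; On BeginPlay it passes DOS to CH_Actor's BindEventToDO, letting the character clear the highlight.
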(event `self.ReceiveBeginPlay`
  (bind _asch_actor (cast `/Game/Self/Character/CH_Actor` (`GameplayStatics.GetPlayerCharacter` 0)))
  (add `/Game/Self/Character/CH_Actor.DO` _asch_actor (delegate `DOS`)))

(event `DOS`
  (`MeshComponent.SetOverlayMaterial` (`self.Knife`) null))

(event `self.Knife.OnComponentBeginOverlap`
  (params (OverlappedComponent :type "PrimitiveComponent Object Reference") (OtherActor :type "Actor Object Reference") (OtherComp :type "PrimitiveComponent Object Reference") (OtherBodyIndex :type Integer) (bFromSweep :type Boolean) (SweepResult :type "HitResult Structure (by ref)"))
  (bind _returnvalue (`GameplayStatics.GetPlayerCharacter` 0))
  (bind _st (`self.ST`))
  ;[1 1 1] Resuable Select Object
  (if (== OtherActor _returnvalue)
    (`MeshComponent.SetOverlayMaterial` (`self.Knife`) "/Game/Self/Textures/Selected.Selected")
    (set `self.Tags` _st)
    (set `ActorComponent.ComponentTags` _st (`self.Knife`))
    (bind _asch_actor (cast `/Game/Self/Character/CH_Actor` _returnvalue))
    (`SceneComponent.SetVisibility` (`/Game/Self/Character/CH_Actor.KCT` _asch_actor) true false)))

(event `self.Knife.OnComponentEndOverlap`
  (params (OverlappedComponent :type "PrimitiveComponent Object Reference") (OtherActor :type "Actor Object Reference") (OtherComp :type "PrimitiveComponent Object Reference") (OtherBodyIndex :type Integer))
  (bind _ust (`self.UST`))
  ;[1 1 1] Resuable Select Object
  (if (== OtherActor (`GameplayStatics.GetPlayerCharacter` 0))
    (`MeshComponent.SetOverlayMaterial` (`self.Knife`) null)
    (set `self.Tags` _ust)
    (set `ActorComponent.ComponentTags` _ust (`self.Knife`))
    (bind _asch_actor (cast `/Game/Self/Character/CH_Actor` (`GameplayStatics.GetPlayerCharacter` 0)))
    (`SceneComponent.SetVisibility` (`/Game/Self/Character/CH_Actor.KCT` _asch_actor) false false)))

(fn `UserConstructionScript`)