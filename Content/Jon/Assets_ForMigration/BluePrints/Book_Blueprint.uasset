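; Book prop Blueprint that gives its static mesh a randomly chosen material when play begins.
; A random MultiGate on BeginPlay picks one output to set the Material variable, which is then applied to the mesh's first material slot.
; Copper and green materials are each wired to two outputs, doubling their odds against the others.
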(event `self.ReceiveBeginPlay`
  (`|MultiGate` true
    (:`Out 0`
      (set `self.Material` "/Game/StarterContent/Materials/M_Metal_Copper.M_Metal_Copper" :!label _label))
    (:`Out 1`
      (goto _label))
    (:`Out 2`
      (set `self.Material` "/Game/StarterContent/Materials/M_Metal_Rust.M_Metal_Rust"))
    (:`Out 3`
      (set `self.Material` "/Game/Jon/Assets_ForMigration/Materials/KnifeMat/KnifeMat2.KnifeMat2"))
    (:`Out 4`
      (set `self.Material` "/DatasmithContent/Materials/FBXImporter/VRED/MetallicCarpaint.MetallicCarpaint"))
    (:`Out 5`
      (set `self.Material` "/Game/InfinityBladeEffects/Maps/LevelContent/Architecture/M_CycWall_01.M_CycWall_01"))
    (:`Out 6`
      (set `self.Material` "/AnimationSharing/AnimSharingRed.AnimSharingRed"))
    (:`Out 7`
      (set `self.Material` "/DatasmithContent/Materials/FBXImporter/VRED/BrushedMetal.BrushedMetal"))
    (:`Out 8`
      (set `self.Material` "/Game/Jon/Assets_ForMigration/Materials/BookMat/BookCoverMat1.BookCoverMat1"))
    (:`Out 9`
      (set `self.Material` "/Engine/MapTemplates/Sky/M_BlackBackground.M_BlackBackground"))
    (:`Out 10`
      (set `self.Material` "/AnimationSharing/AnimSharingGreen.AnimSharingGreen" :!label _label_2))
    (:`Out 11`
      (goto _label_2)))
  (`PrimitiveComponent.SetMaterial` (`self.StaticMesh`) 0 (`self.Material`)))

(fn `UserConstructionScript`)