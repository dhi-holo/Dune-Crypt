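; A fire pit actor that lights when the player character walks into its trigger box.
; The overlap toggles the visibility of a blue torch fire component and destroys the box, so it fires only once.
; An ignition sound plays at the sphere component's location, followed by a crackling fire sound there after a short delay.
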(event `self.Box.OnComponentBeginOverlap`
  (params (OverlappedComponent :type "PrimitiveComponent Object Reference") (OtherActor :type "Actor Object Reference") (OtherComp :type "PrimitiveComponent Object Reference") (OtherBodyIndex :type Integer) (bFromSweep :type Boolean) (SweepResult :type "HitResult Structure (by ref)"))
  (if (== OtherActor (`GameplayStatics.GetPlayerCharacter` 0))
    (`SceneComponent.ToggleVisibility` (`self.P_Fire_Torch_Blue`) false)
    (`ActorComponent.K2_DestroyComponent` (`self.Box`))
    (`GameplayStatics.PlaySoundAtLocation` "/Game/Self/Sound/lighting-a-fire-14421.lighting-a-fire-14421" (`SceneComponent.K2_GetComponentLocation` (`self.Sphere`)) (struct) 1.0 1.0 0.0 null null null null)
    (`KismetSystemLibrary.Delay` 0.2)
    (`GameplayStatics.PlaySoundAtLocation` "/Game/Self/Sound/crackling-fire-14759.crackling-fire-14759" (`SceneComponent.K2_GetComponentLocation` (`self.Sphere`)) (struct) 1.0 1.0 0.0 null null null null)))

(fn `UserConstructionScript`)